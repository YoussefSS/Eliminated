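; Blueprint for an AI-controlled guard character driven by the BT_AICharacter behavior tree.
; BeginPlay runs the tree and seeds blackboard values for patrol-guard status, the next patrol point, and original location and rotation.
; A timeline lerps actor rotation along the shortest path for the tree's look-back-to-original-rotation step.
; Death stops the brain logic, while perception updates pass straight to the parent class.
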(event `self.ReceiveTick`
  (params (DeltaSeconds :type "Float (single-precision)")))

(event `self.LookAtRotationOverTime`
  (params (RotToLookAt :type "Rotator Structure"))
  ;[1 1 1] Look At Original Rotation (from BT)
  (bind (_direction _rotationalpha) (`Timeline|LookAtRotation`)
    (:`Update`
      (`self.K2_SetActorRotation` (`KismetMathLibrary.RLerp` (`self.K2_GetActorRotation`) RotToLookAt _rotationalpha true)))))

(event `self.ReceiveBeginPlay`
  (`|ExecutionSequence`
    (:`then_0`
      ;[1 1 1] Running Behavior Tree
      (`AIController.RunBehaviorTree` (`AIBlueprintHelperLibrary.GetAIController` self) "/Game/AI/BT_AICharacter.BT_AICharacter"))
    (:`then_1`
      ;[1 1 1] Setting Initial BB Values
      (`self.SetIsPatrolGuardBBValue`)
      (`self.GetNextPatrolPointAndSetBBValues`)
      (`self.SetOriginalLocationAndRotationBBValues`))))

(event `self.OnDeath`
  ;[1 1 1] On Death
  (`BrainComponent.StopLogic` (`AIController.BrainComponent` (`AIBlueprintHelperLibrary.GetAIController` self)) "Dead"))

(event `self.OnPerceptionUpdated`
  (params (UpdatedActors :type "Array of Actor Object Reference (by ref)"))
  ;[1 1 1] Perception Updated
  (`parent.OnPerceptionUpdated` UpdatedActors))

(fn `UserConstructionScript`)
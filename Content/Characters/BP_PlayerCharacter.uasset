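; Player character Blueprint that handles the camera transition for aiming down sights.
; Start and stop events play and reverse a timeline, whose alpha blends the spring arm's length and socket offset between regular and aiming values.
; A debug key on B prints the character's horizontal speed.
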(event `self.StartAimDownSights_Event`
  (bind _cameraboom (`self.CameraBoom`))
  ;[1 1 1] Aiming Down Sights
  (bind (_direction _aimdownsightalpha) (`Timeline|AimDownSights_Timeline` :!label _label)
    (:`Update`
      (set `SpringArmComponent.TargetArmLength` (`KismetMathLibrary.Lerp` (`self.SpringArmDistance_AimDownSight`) (`self.SpringArmDistance_Regular`) _aimdownsightalpha) _cameraboom)
      (set `SpringArmComponent.SocketOffset` (`KismetMathLibrary.VLerp` (`self.SpringArmCameraOffset_AimDownSight`) (0.0 0.0 0.0) _aimdownsightalpha) _cameraboom))))

(event `self.StopAimDownSights_Event`
  ;[1 1 1] Aiming Down Sights
  (goto _label :!via `Reverse`))

(event `Key|B`
  (params (Key :type "Key Structure"))
  (bind (_returnvalue_x _returnvalue_y) (`KismetMathLibrary.BreakVector` (`self.GetVelocity`)))
  (:`Pressed`
    (`KismetSystemLibrary.PrintString` (`KismetStringLibrary.Concat_StrStr` "Velocity" (`KismetStringLibrary.Conv_DoubleToString` (`KismetMathLibrary.VSize` (`KismetMathLibrary.MakeVector` _returnvalue_x _returnvalue_y)))))))

(fn `UserConstructionScript`)